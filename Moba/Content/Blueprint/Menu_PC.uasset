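; Main menu PlayerController that shows the menu widget with a visible cursor and handles multiplayer session hosting and joining.
; Heberger creates a four-slot non-LAN session and opens MainMap as a listen server.
; Rechercher fills the widget's session list with one HUD_Session entry per search result, toggling IsFinding around the search.
; JoinSession joins a given result, while Rejoindre connects by IP through an open console command.
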(event `self.ReceiveBeginPlay`
  ;[1 1 1] Initialisation
  (`self.HUD_Menu`)
  (`self.Init Cursor`))

(event `HUD_Menu`
  ;[1 1 1] Affichage De HUD menu
  (`/Engine/EditorBlueprintResources/StandardMacros.IsValid` (`self.HUV_Menu_Var`)
    (:`Is Not Valid`
      (bind _returnvalue (`|CreateWidget` "/Game/UI/HUD_Menu.HUD_Menu_C"))
      (bind _output_get (set `self.HUV_Menu_Var` _returnvalue))
      (`UserWidget.AddToViewport` _output_get 0))))

(event `Init Cursor`
  ;[1 1 1] Init cursor
  (set `self.bShowMouseCursor` true)
  (`WidgetBlueprintLibrary.SetInputMode_GameAndUIEx` self null "LockAlways" false))

(event `Heberger`
  ;[1 1 1] Heberger
  (`CreateSessionCallbackProxy.CreateSession` self 4
    (:`OnSuccess`
      (`GameplayStatics.OpenLevel` "MainMap" true "listen"))))

(event `Rejoindre`
  (params (IP :type String))
  ;[1 1 1] Rejoindre
  (`KismetSystemLibrary.ExecuteConsoleCommand` (`KismetStringLibrary.Concat_StrStr` "open " IP) null))

(event `Rechercher`
  (`PanelWidget.ClearChildren` (`/Game/UI/HUD_Menu.Lst_Session` (`self.HUV_Menu_Var`)))
  (set `self.IsFinding` true)
  (bind _results (`FindSessionsCallbackProxy.FindSessions` self 10)
    (:`then`
      (for _array_element _results
        (`|CreateWidget` "/Game/UI/HUD_Session.HUD_Session_C" null _array_element)
        (`PanelWidget.AddChild` (`/Game/UI/HUD_Menu.Lst_Session` (`self.HUV_Menu_Var`)) null))
      (set `self.IsFinding` false))))

(event `Join Session`
  (params (SearchResult :type "BlueprintSessionResult Structure (by ref)"))
  (`JoinSessionCallbackProxy.JoinSession` self SearchResult))

(fn `UserConstructionScript`)